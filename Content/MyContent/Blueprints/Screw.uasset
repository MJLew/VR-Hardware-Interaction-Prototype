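; Screw hardware actor that an ElectricDrill drives in or backs out while it is attached and overlapped by a tool.
; The overlapping drill is cached, and its Screwing flag sets whether Tick counts Completion down or up.
; Each step rolls the mesh, updates grabbability and calls completion at zero or incompletion otherwise.
; Construction starts the screw fully unscrewed and sets its screw interactivity tag.
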(event `self.ReceiveBeginPlay`
  (`parent.ReceiveBeginPlay`))

(event `self.ReceiveActorBeginOverlap`
  (params (OtherActor :type "Actor Object Reference"))
  ;[1 1 1] Overlap Events - When overlapping with a drill, store which drill it is attached to
  (bind _aselectric_drill (cast `/Game/MyContent/Blueprints/ElectricDrill` OtherActor))
  (set `self.currentDrill` _aselectric_drill))

(event `self.ReceiveActorEndOverlap`
  (params (OtherActor :type "Actor Object Reference"))
  ;[1 1 1] Overlap Events - When overlapping with a drill, store which drill it is attached to
  (if (== OtherActor (`self.currentDrill`))
    (set `self.currentDrill` null)))

(event `self.ReceiveTick`
  (params (DeltaSeconds :type "Float (single-precision)"))
  (bind _completion (`self.completion`))
  ;[1 1 1] Tick Events - When drilling count up/down the completion of the screw. Only screws when overlapped with tool and is attached to wall
  (if (and (`self.overlappedTool`) (`self.isAttached`))
    ;;[1 1 1] If screwing in decrement completion. If unscrewing increment completion.
    (if (`/Game/MyContent/Blueprints/ElectricDrill.screwing` (`self.currentDrill`))
      (set `self.incValue` -1)
      (if (> _completion 0)
        (set `self.completion` (+ _completion (`self.incValue`)) :!label _label)
        (`self.Rotate Screw`)
        (`self.SetGrabbable`)
        (bind _output_get (set `self.isCompleted` (== (`self.completion`) 0)))
        (if _output_get
          (`self.onCompletion` self)
          (else
            (`self.onIncompletion` self))))
      (else
        (set `self.incValue` 1)
        (if (<= _completion (`self.completionMax`))
          (goto _label))))))

(fn `Rotate Screw`
  (bind _hardware_sm (`self.Hardware_SM`))
  (`SceneComponent.K2_SetRelativeRotation` _hardware_sm (`KismetMathLibrary.MakeRotator` (+ (.roll (`SceneComponent.RelativeRotation` _hardware_sm)) (* (`self.incValue`) 10)) (.pitch (`SceneComponent.RelativeRotation` _hardware_sm)) (.yaw (`SceneComponent.RelativeRotation` _hardware_sm))) false false))

(fn `UserConstructionScript`
  (`parent.UserConstructionScript`)
  (bind _output_get (set `self.completionMax` 300))
  (set `self.completion` _output_get)
  (set `self.interactivityTag` (struct :`TagName` "ForScrews")))