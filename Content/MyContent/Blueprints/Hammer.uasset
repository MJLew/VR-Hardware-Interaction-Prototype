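; Hammer actor that pulls a Nail out of the wall when held on it for about three seconds.
; Begin overlap stores one nail at a time, and any end overlap clears it and resets the count.
; Tick uses a one-second Delay to raise PullCount, capped by the nail's CompletionMax.
; At three, it calls PullOutFromWall every tick until the count resets.
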(event `self.ReceiveActorBeginOverlap`
  (params (OtherActor :type "Actor Object Reference"))
  ;[1 1 1] Overlap Events - Save the first nail the hammer overlaps. (Can hammer multiple nails, but can only pull out one at a time)
  (bind _asnail (cast `/Game/MyContent/Blueprints/Nail` OtherActor))
  (if (not (`self.hasCurrentNail`))
    (set `self.currentNail` _asnail)))

(event `self.ReceiveActorEndOverlap`
  (params (OtherActor :type "Actor Object Reference"))
  ;[1 1 1] End Overlap Events - Detach current nail and reset pull count timer
  (set `self.currentNail` null)
  (set `self.pullCount` 0))

(event `self.ReceiveTick`
  (params (DeltaSeconds :type "Float (single-precision)"))
  (bind _currentnail (`self.currentNail`))
  ;[1 1 1] Tick Events - If holding hammer on nail for 3 seconds, reset the nail's completion. Otherwise continue counting to 3
  (if (>= (`self.pullCount`) 3)
    (`/Game/MyContent/Blueprints/Nail.Pull Out From Wall` _currentnail)
    (else
      ;;[1 1 1] Count to 3
      (if (and (`self.hasCurrentNail`) (< (`self.pullCount`) (`/Game/MyContent/Blueprints/Hardware_Base.completionMax` _currentnail)))
        (`KismetSystemLibrary.Delay` 1.0)
        (set `self.pullCount` (+ (`self.pullCount`) 1))))))

(fn `UserConstructionScript`
  (`parent.UserConstructionScript`)
  (`StaticMeshComponent.SetStaticMesh` (`self.StaticMesh`) "/Game/MS_MedievalTools/3D_Assets/Blacksmith_Hammer_00/ueqjee3fa_LOD0.ueqjee3fa_LOD0"))