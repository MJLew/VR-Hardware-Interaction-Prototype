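; WallInteractPoint is a wall interaction point that holds one Hardware_Base object and tracks whether it is completed.
; AttachHardware accepts hardware when none is attached and binds to its completion and incompletion events, with handlers that set IsCompleted.
; When the attached hardware leaves the collision component, it is detached and its events are unbound.
; Overlap begin does nothing, so attachment relies on a call to AttachHardware.
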(event `self.CollisionComponent.OnComponentBeginOverlap`
  (params (OverlappedComponent :type "PrimitiveComponent Object Reference") (OtherActor :type "Actor Object Reference") (OtherComp :type "PrimitiveComponent Object Reference") (OtherBodyIndex :type Integer) (bFromSweep :type Boolean) (SweepResult :type "HitResult Structure (by ref)")))

(event `self.CollisionComponent.OnComponentEndOverlap`
  (params (OverlappedComponent :type "PrimitiveComponent Object Reference") (OtherActor :type "Actor Object Reference") (OtherComp :type "PrimitiveComponent Object Reference") (OtherBodyIndex :type Integer))
  (if (== OtherActor (`self.attachedHardware`))
    (`self.detachHardware`)))

(fn `attachHardware`
  (params (Object :type "Object Object Reference"))
  (bind _ashardware_base (cast `/Game/MyContent/Blueprints/Hardware_Base` Object))
  (if (not (`self.hasHardwareAttached`))
    (bind _output_get (set `self.attachedHardware` _ashardware_base))
    (add `/Game/MyContent/Blueprints/Hardware_Base.onCompletion` _output_get (`|CreateDelegate` self :!event `bind_On Hardware Completion`))
    (add `/Game/MyContent/Blueprints/Hardware_Base.onIncompletion` _output_get (`|CreateDelegate` self :!event `bind_On Hardware Incompletion`))))

(fn `bind_On Hardware Completion`
  (set `self.isCompleted` true))

(fn `bind_On Hardware Incompletion`
  (set `self.isCompleted` false))

(fn `detachHardware`
  (bind _attachedhardware (`self.attachedHardware`))
  (clear `/Game/MyContent/Blueprints/Hardware_Base.onCompletion` _attachedhardware)
  (clear `/Game/MyContent/Blueprints/Hardware_Base.onIncompletion` _attachedhardware)
  (set `self.attachedHardware` null))

(fn `UserConstructionScript`)