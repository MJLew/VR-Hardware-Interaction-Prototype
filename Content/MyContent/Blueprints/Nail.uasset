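; Nail hardware piece that hammers drive into a wall over several hits.
; While attached, each Hammer overlap decrements a completion counter, refreshes grabbability and nudges the mesh along its forward axis, calling OnCompletion at zero.
; PullOutFromWall resets the counter, refreshes grabbability, nudges the mesh the opposite way and calls OnIncompletion.
; The construction script initializes the counter and tags the nail for nail-specific interactions.
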(event `self.ReceiveBeginPlay`
  (`parent.ReceiveBeginPlay`))

(event `self.ReceiveActorBeginOverlap`
  (params (OtherActor :type "Actor Object Reference"))
  (bind _completion (`self.completion`))
  ;[1 1 1] Overlap Events - If overlapped by a hammer AND is attached to a wall AND completion above 0, progress completion
  (cast `/Game/MyContent/Blueprints/Hammer` OtherActor)
  (if (and (`self.isAttached`) (> _completion 0))
    (set `self.completion` (- _completion 1))
    (`self.SetGrabbable`)
    (`self.Move Nail When Hit` -1.0)
    (bind _output_get (set `self.isCompleted` (== (`self.completion`) 0)))
    (if _output_get
      (`self.onCompletion`))))

(fn `Move Nail When Hit`
  (params (movementScale :type "Float (double-precision)"))
  (bind _hardware_sm (`self.Hardware_SM`))
  (`SceneComponent.K2_AddWorldOffset` _hardware_sm (* (`SceneComponent.GetForwardVector` _hardware_sm) (`KismetMathLibrary.MakeVector` movementScale movementScale movementScale)) false false))

(fn `Pull Out From Wall`
  (set `self.completion` (`self.completionMax`))
  (`self.SetGrabbable`)
  (`self.Move Nail When Hit` 0.3)
  (set `self.isCompleted` false)
  (`self.onIncompletion`))

(fn `UserConstructionScript`
  (`parent.UserConstructionScript`)
  (bind _output_get (set `self.completionMax` 3))
  (set `self.completion` _output_get)
  (set `self.interactivityTag` (struct :`TagName` "ForNails")))