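; Base Blueprint for grabbable hardware that the player can drop onto wall interact points to attach it.
; Grab component drop and grab events drive attaching to the first overlapping point with a matching interactivity tag, and detaching again.
; Attaching notifies the wall point, while detaching only clears the hardware's own reference and flag.
; SetGrabbable switches the grab type based on whether Completion has reached its maximum.
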(event `self.ReceiveBeginPlay`
  (bind _grabcomponent (`self.GrabComponent`))
  (add `/Game/VRTemplate/Blueprints/GrabComponent.OnDropped` _grabcomponent (delegate `onDropped_bind`))
  (add `/Game/VRTemplate/Blueprints/GrabComponent.OnGrabbed` _grabcomponent (delegate `onGrabbed_bind`)))

(event `onDropped_bind`
  ;[1 1 1] Bound GrabComponent Event - If dropped, check if should attach to wall
  (`self.AttachToWall`))

(event `onGrabbed_bind`
  ;[1 1 1] Bound GrabComponent Event - If grabbed detach from wall
  (`self.DetachFromWall`))

(fn `AttachToWall`
  ;[1 1 1] When the hardware is dropped on a wall interact point, attach and remember that point
  (bind _aswall_interact_point (cast `/Game/MyContent/Blueprints/WallInteractPoint` (`|GetArrayItem` (`PrimitiveComponent.GetOverlappingActors` (`self.CapsuleCollision`) "/Game/MyContent/Blueprints/WallInteractPoint.WallInteractPoint_C"))))
  (if (== (`/Game/MyContent/Blueprints/WallInteractPoint.interactivityTag` _aswall_interact_point) (`self.interactivityTag`))
    (bind _output_get (set `self.attachedWallPoint` _aswall_interact_point))
    (`/Game/MyContent/Blueprints/WallInteractPoint.attachHardware` _output_get self)
    (set `self.isAttached` true)))

(fn `DetachFromWall`
  (set `self.attachedWallPoint` null)
  (set `self.isAttached` false))

(fn `SetGrabbable`
  (bind _grabcomponent (`self.GrabComponent`))
  (if (< (`self.completion`) (`self.completionMax`))
    (set `/Game/VRTemplate/Blueprints/GrabComponent.GrabType` "NewEnumerator0" _grabcomponent)
    (else
      (set `/Game/VRTemplate/Blueprints/GrabComponent.GrabType` "NewEnumerator4" _grabcomponent))))

(fn `UserConstructionScript`)