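; Electric drill tool actor that works on Screw actors, with its drill mesh assigned in the construction script.
; Actor overlap caches the overlapped screw and sets its OverlappedTool flag, clearing both when that screw leaves the overlap.
; The trigger toggles direction through the Screwing flag: pressing sets it to unscrew, releasing returns it to the default of screwing in.
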(event `self.ReceiveActorBeginOverlap`
  (params (OtherActor :type "Actor Object Reference"))
  ;[1 1 1] Overlap Events - Get the overlapped screw and set its "Overlapped Tool" variable to True/False
  (bind _asscrew (cast `/Game/MyContent/Blueprints/Screw` OtherActor))
  (bind _output_get (set `self.currentScrew` _asscrew))
  (set `/Game/MyContent/Blueprints/Hardware_Base.overlappedTool` true _output_get))

(event `self.ReceiveActorEndOverlap`
  (params (OtherActor :type "Actor Object Reference"))
  (bind _currentscrew (`self.currentScrew`))
  ;[1 1 1] Overlap Events - Get the overlapped screw and set its "Overlapped Tool" variable to True/False
  (if (== OtherActor _currentscrew)
    (set `/Game/MyContent/Blueprints/Hardware_Base.overlappedTool` false _currentscrew)
    (set `self.currentScrew` null)))

(event `/Game/VRTemplate/Blueprints/VRInteractionBPI.TriggerPressed`
  ;[1 1 1] If pressing the primary trigger while holding, unscrews. Screws in by default
  (set `self.screwing` false))

(event `/Game/VRTemplate/Blueprints/VRInteractionBPI.TriggerReleased`
  ;[1 1 1] If pressing the primary trigger while holding, unscrews. Screws in by default
  (set `self.screwing` true))

(fn `UserConstructionScript`
  (`parent.UserConstructionScript`)
  (`StaticMeshComponent.SetStaticMesh` (`self.StaticMesh`) "/Game/Construction_VOL2/Meshes/SM_ElectricDrill_01a.SM_ElectricDrill_01a"))